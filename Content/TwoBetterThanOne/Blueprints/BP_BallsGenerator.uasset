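; Networked ball generator that spawns a ball on interaction and starts movement when a car trigger activates.
; Both events branch on authority: the authority calls the spawn or movement RPC directly, while remote instances route through a matching server RPC.
; Those RPCs call SpawnBall and StartMovement, whose logic is not defined in these graphs.
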(event Custom|RPC_Server_SpawnBall
  ;[1 1 1] Spawn ball
  (CallFunction|RPCSpawnBall))

(event Custom|RPC_SpawnBall
  ;[1 1 1] Spawn ball
  (Class|BallsGenerator|SpawnBall))

(event Custom|RPC_Server_StartMovement
  ;[1 1 1] Start movement
  (CallFunction|RPCStartMovement))

(event Custom|RPC_StartMovement
  ;[1 1 1] Start movement
  (Class|BallsGenerator|StartMovement))

(event EventBeginPlay)

(event Collision|EventActorBeginOverlap
  (params (OtherActor :type Actor%20Object%20Reference)))

(event EventTick
  (params (DeltaSeconds :type Float%20%28single-precision%29)))

(event EventNotifyInteraction
  ;[1 1 1] Spawn ball
  (Networking|SwitchHasAuthority
    (:Authority
      (CallFunction|RPCSpawnBall))
    (:Remote
      (CallFunction|RPCServerSpawnBall))))

(event EventCarTriggerActivated
  ;[1 1 1] Start movement
  (Networking|SwitchHasAuthority
    (:Authority
      (CallFunction|RPCStartMovement))
    (:Remote
      (CallFunction|RPCServerStartMovement))))

(fn ConstructionScript)