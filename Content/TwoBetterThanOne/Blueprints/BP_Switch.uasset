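; BP_Switch is an interactable switch that the player can trigger to act on a linked Target actor.
; When an actor tagged Player enters the Collider, it shows ActionText and passes itself to that player by message; leaving hides the text and notifies the player.
; On NotifyInteraction, it forwards an interaction message to Target if valid, so the switch stays decoupled from what it activates.
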(event OnComponentBeginOverlap(Collider)
  (params (OverlappedComponent :type Primitive%20Component%20Object%20Reference) (OtherActor :type Actor%20Object%20Reference) (OtherComp :type Primitive%20Component%20Object%20Reference) (OtherBodyIndex :type Integer) (bFromSweep :type Boolean) (SweepResult :type Hit%20Result%20Structure%20%28by%20ref%29))
  (if (Actor|ActorHasTag OtherActor "Player")
    (Rendering|SetVisibility (Variables|Default|GetActionText) true false)
    (Class|SwitchInterface|IsonTrigger(Message) OtherActor self)))

(event OnComponentEndOverlap(Collider)
  (params (OverlappedComponent :type Primitive%20Component%20Object%20Reference) (OtherActor :type Actor%20Object%20Reference) (OtherComp :type Primitive%20Component%20Object%20Reference) (OtherBodyIndex :type Integer))
  (if (Actor|ActorHasTag OtherActor "Player")
    (Rendering|SetVisibility (Variables|Default|GetActionText) false false)
    (Class|SwitchInterface|OutOfTrigger(Message) OtherActor)))

(event EventBeginPlay)

(event Collision|EventActorBeginOverlap
  (params (OtherActor :type Actor%20Object%20Reference)))

(event EventTick
  (params (DeltaSeconds :type Float%20%28single-precision%29)))

(event EventNotifyInteraction
  (bind _target (Variables|Default|GetTarget))
  (Utilities|IsValid _target
    (:Is%20Valid
      (Class|SwitchInterface|NotifyInteraction(Message) _target))))

(fn ConstructionScript)